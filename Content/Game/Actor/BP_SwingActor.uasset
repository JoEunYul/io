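; BP_SwingActor is an obstacle actor that swings its Center component back and forth around the roll axis.
; On BeginPlay, the Swing timeline drives Center's relative roll, scaled to 45 degrees, and toggles IsRun on finish to alternate between Play and Reverse.
; The Sphere hit event casts to BP_GameCharactor but does nothing further.
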(event `self.ReceiveBeginPlay`
  (if (`self.is run`) :!label _label
    (bind (_direction `_새_트랙_0`) (`Timeline|swing` :`NewTime` 0.01 :!label _label_2)
      (:`Update`
        (`SceneComponent.K2_SetRelativeRotation` (`self.Center`) (`KismetMathLibrary.MakeRotator` (* `_새_트랙_0` 45.0)) false false))
      (:`Finished`
        (set `self.is run` (not (`self.is run`)))
        (goto _label)))
    (else
      (goto _label_2 :!via `Reverse`))))

(event `self.Sphere.OnComponentHit`
  (params (HitComponent :type "PrimitiveComponent Object Reference") (OtherActor :type "Actor Object Reference") (OtherComp :type "PrimitiveComponent Object Reference") (NormalImpulse :type "Vector Structure") (Hit :type "HitResult Structure (by ref)"))
  (cast `/Game/Game/BP_GameCharactor` OtherActor))

(fn `UserConstructionScript`)