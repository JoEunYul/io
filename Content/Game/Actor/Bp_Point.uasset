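; Bp_Point is a point pickup actor whose cube spins and bobs in place.
; A looping timer calls Move, which yaws the cube through MoveRotate.
; A timeline drives the cube's relative Z, with IsRight flipped on finish to alternate Play and Reverse.
; Any overlap on the cube prints "Get Point" and hides the actor, without destroying it or adding score.
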(event `self.ReceiveBeginPlay`
  (`KismetSystemLibrary.K2_SetTimer` null "Move" 0.01 true)
  (if (`self.Is Right`) :!label _label
    (bind (_direction `_새_트랙_0`) (`Timeline|타임라인_0` :!label _label_2)
      (:`Update`
        (`SceneComponent.K2_SetRelativeLocation` (`self.Cube`) (`KismetMathLibrary.MakeVector` 0.0 0.0 (* `_새_트랙_0` 10.0)) false false))
      (:`Finished`
        (set `self.Is Right` (not (`self.Is Right`)))
        (goto _label)))
    (else
      (goto _label_2 :!via `Reverse`))))

(event `self.Cube.OnComponentBeginOverlap`
  (params (OverlappedComponent :type "PrimitiveComponent Object Reference") (OtherActor :type "Actor Object Reference") (OtherComp :type "PrimitiveComponent Object Reference") (OtherBodyIndex :type Integer) (bFromSweep :type Boolean) (SweepResult :type "HitResult Structure (by ref)"))
  (`KismetSystemLibrary.PrintString` "Get Point")
  (`self.SetActorHiddenInGame` true))

(fn `Move`
  (`self.MoveRotate` 0.01))

(fn `MoveRotate`
  (params (Speed :type "Float (double-precision)"))
  (`SceneComponent.K2_AddLocalRotation` (`self.Cube`) (`KismetMathLibrary.MakeRotator` 0.0 0.0 (* Speed 50.0)) false false))

(fn `UserConstructionScript`)