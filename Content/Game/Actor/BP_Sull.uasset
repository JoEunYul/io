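; BP_Sull is an actor that slides its static mesh along the Z axis in small steps.
; A fast looping timer started on BeginPlay calls Move, which passes a fixed speed to SnowBoard.
; SnowBoard raises the mesh while IsRight is set, then clears the flag once relative Z passes an upper limit.
; The other branch applies a derived Z offset, but its below-zero check does nothing, so IsRight is never set again.
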(event `self.ReceiveBeginPlay`
  (`KismetSystemLibrary.K2_SetTimer` null "Move" 0.01 true))

(fn `Move`
  (`self.SnowBoard` 0.01))

(fn `SnowBoard`
  (params (Speed :type "Float (double-precision)"))
  (bind _returnvalue (* Speed 150.0))
  (bind _staticmesh (`self.StaticMesh`))
  (bind (_relativelocation_x _relativelocation_y _relativelocation_z) (`KismetMathLibrary.BreakVector` (`SceneComponent.RelativeLocation` _staticmesh)))
  (bind (_relativelocation_x_2 _relativelocation_y_2 _relativelocation_z_2) (`KismetMathLibrary.BreakVector` (`SceneComponent.RelativeLocation` _staticmesh)))
  (if (`self.Is Right`)
    (`SceneComponent.K2_AddWorldOffset` _staticmesh (`KismetMathLibrary.MakeVector` 0.0 0.0 _returnvalue) false false)
    (if (< 300.0 _relativelocation_z_2)
      (set `self.Is Right` false))
    (else
      (bind _result (`/Engine/EditorBlueprintResources/StandardMacros.NegateFloat` _returnvalue)
        (:`  `
          (`SceneComponent.K2_AddWorldOffset` _staticmesh (`KismetMathLibrary.MakeVector` 0.0 0.0 _result) false false)
          (if (< _relativelocation_z 0.0)
            (if true
              _)))))))

(fn `UserConstructionScript`)